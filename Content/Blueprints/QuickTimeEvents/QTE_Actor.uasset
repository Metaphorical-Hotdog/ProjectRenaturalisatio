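; Interactable actor that runs a quick-time event minigame for the player, disabling their input until it ends.
; Each round puts a QTE_HUD2 with a random input and time limit on its widget component, sized to the draw size.
; A success re-fires the OnNotEnough dispatcher for another round until three are counted.
; Completion or failure prints the result and restores input; failure leaves the success count intact.
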(event `/Game/Blueprints/Interfaces/BPI_Interactable.Interact`
  (params (Instigator :type "/Game/Blueprints/Characters/BP_Character_Base Object Reference"))
  (`self.DisableInput` Instigator null)
  (`/Game/Blueprints/QuickTimeEvents/BPI_EventManager.QTEGameStart` Instigator))

(event `OnNotEnough_Event`
  (bind (_returnvalue_x _returnvalue_y) (`KismetMathLibrary.BreakVector2D` (`WidgetComponent.GetDrawSize` (`self.Widget`))))
  (bind _sizebox_37 (`/Game/Blueprints/QuickTimeEvents/QTE_HUD2.SizeBox_37` (`self.QTEWidgetRef2`)))
  (if (and (== (stale `/Game/Blueprints/QuickTimeEvents/BPI_EventManager.QTEGameStart` ActorTarget) (`GameplayStatics.GetPlayerCharacter` 0)) (not (`self.IsActive`))) :!label _label
    (add `self.OnNotEnough` (delegate `OnNotEnough_Event`))
    (bind _returnvalue (`|CreateWidget` "/Game/Blueprints/QuickTimeEvents/QTE_HUD2.QTE_HUD2_C" null (`KismetArrayLibrary.Array_Random` (`|MakeArray` "NewEnumerator0" "NewEnumerator1" "NewEnumerator2" "NewEnumerator3" :!type "/Game/Blueprints/QuickTimeEvents/E_QuickTimeInputs Enum")) (`self.TimeToReact`)))
    (`WidgetComponent.SetWidget` (`self.Widget`) _returnvalue)
    (bind _output_get (set `self.QTEWidgetRef2` _returnvalue))
    (add `/Game/Blueprints/QuickTimeEvents/QTE_HUD2.FinishedQTE` _output_get (`|CreateDelegate` :!event `FinishedQTE_Event`))
    (set `self.IsActive` true)
    (`SizeBox.SetHeightOverride` _sizebox_37 _returnvalue_y)
    (`SizeBox.SetWidthOverride` _sizebox_37 _returnvalue_x)))

(event `/Game/Blueprints/QuickTimeEvents/BPI_EventManager.QTEGameStart`
  (params (ActorTarget :type "Actor Object Reference"))
  (goto _label))

(event `FinishedQTE_Event`
  (params (Success :type Boolean))
  (set `self.IsActive` false)
  (clear `/Game/Blueprints/QuickTimeEvents/QTE_HUD2.FinishedQTE` (`self.QTEWidgetRef2`))
  (`WidgetComponent.SetWidget` (`self.Widget`) null)
  (set `self.QTEWidgetRef2` null)
  (if Success
    (`/Engine/EditorBlueprintResources/StandardMacros.IncrementInt` (`self.SuccessCounter`)
      (:`  `
        (if (== (`self.SuccessCounter`) 3)
          (`KismetSystemLibrary.PrintString` "Success")
          (`WidgetComponent.SetWidget` (`self.Widget`) null)
          (set `self.SuccessCounter` 0)
          (`KismetSystemLibrary.Delay` 0.2)
          (`self.EnableInput` (`GameplayStatics.GetPlayerCharacter` 0) null)
          (remove `self.OnNotEnough` (`|CreateDelegate` :!event `OnNotEnough_Event`))
          (else
            (`self.OnNotEnough`)))))
    (else
      (`KismetSystemLibrary.PrintString` "FAILURE")
      (`WidgetComponent.SetWidget` (`self.Widget`) null)
      (`KismetSystemLibrary.Delay` 0.2)
      (`self.EnableInput` (`GameplayStatics.GetPlayerCharacter` 0) null))))

(fn `QTEGameFinished`
  (returns (Success :type Boolean))
  (return false))

(fn `ShowNextLine`
  (returns (HasNextLine :type Boolean))
  (return false))

(fn `UserConstructionScript`)