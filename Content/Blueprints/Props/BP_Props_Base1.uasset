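; Base interactable prop that runs a quick-time event and, after three successes, turns into grass and shows dialogue.
; ChildInteraction locks player input and spawns randomized QTE widgets; success triggers RevealNature and DT_Dialogue lines on the HUD.
; RevealNature swaps the mesh and grows a sphere mask through timelines driving indexed MPC_MaskingNature parameters.
; Masks are recorded in GM_Solar's array, which SavedNature uses to regrow revealed props.
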(event `self.ReceiveBeginPlay`
  ;[1 1 1] This is to cast shadows on the Dialogue Widget
  (`PrimitiveComponent.SetCastShadow` (`self.DialogueIndicator`) false)
  (set `self.Reset Row Name` (`self.Current Row Name`))
  ;[1 1 1] This is to set a reference to Game Instance and Mode for all Props
  (bind _asgi_solar (cast `/Game/Blueprints/GI_Solar` (`GameplayStatics.GetGameInstance`)))
  (set `self.GameInstance` _asgi_solar)
  (bind _asgm_solar (cast `/Game/Blueprints/GM_Solar` (`GameplayStatics.GetGameMode`)))
  (set `self.GameMode` _asgm_solar))

(event `self.ReceiveTick`
  (params (DeltaSeconds :type "Float (single-precision)"))
  (set `self.Delta Seconds` DeltaSeconds))

(event `Child Interaction`
  (params (Instigator :type "/Game/Blueprints/Characters/BP_Character_Base Object Reference"))
  ;[1 1 1] Display Dialogue through Interface
  (if (and (!= (`self.Current Row Name`) "None") (`self.IsInteractable`))
    (`self.QTEGameStart` Instigator)
    (set `self.PlayerInstigates` Instigator)
    (`self.DisableInput` Instigator (`GameplayStatics.GetPlayerController` 0))
    (else
      (`GameplayStatics.PlaySound2D` "/Game/Sounds/S_Ambience_General_Cue.S_Ambience_General_Cue" 1.0 1.0 0.0 null null))))

(event `self.FinishInteraction`
  ;[1 1 1] Ends the interaction, the rest is handled on BP Player
  (`self.EndInteraction`))

(event `RevealNature`
  (bind _gamemode (`self.GameMode`))
  (bind _gamemode_2 (`self.GameMode`))
  (bind _gamemode_3 (`self.GameMode`))
  (bind _natureindex (`/Game/Blueprints/GM_Solar.NatureIndex` _gamemode))
  (bind _natureindex_2 (`/Game/Blueprints/GM_Solar.NatureIndex` (`self.GameMode`)))
  (bind _returnvalue (`KismetMathLibrary.Conv_VectorToLinearColor` (`SceneComponent.K2_GetComponentLocation` (`self.SM_wood_box_01`))))
  ; Increase the radius of the sphere mask so that the second texture takes over and the static mesh changes.
  (`StaticMeshComponent.SetStaticMesh` (`self.SM_wood_box_01`) "/Game/Maps/Materials/Landscape/grass/SM_Grass2.SM_Grass2")
  (`PrimitiveComponent.SetMaterial` (`self.SM_wood_box_01`) 0 "/Game/Maps/StylizedProvencal/Materials/MI_GrassField.MI_GrassField")
  (for _ (`self.MaskingCenterArray`) :!label _label
    (for _array_element (`/Game/Blueprints/GM_Solar.NatureSphereMasks` _gamemode)
      (bind _output (`self.GetMaskCenterArray` _natureindex))
      (bind _output_2 (`self.GetMaskRadiusArray` _natureindex))
      (if (not (`KismetStringLibrary.EqualEqual_StrStr` (break `/Game/DataTables/Masking/S_NatureMask` _array_element)))
        (if (not (and (`KismetStringLibrary.EqualEqual_StrStr` (break `/Game/DataTables/Masking/S_NatureMask` _array_element) (`KismetSystemLibrary.GetDisplayName` self)) (== (`.MaskName_5_AA23EB1444594C3974AFD4A2287DAFA3` (break `/Game/DataTables/Masking/S_NatureMask` _array_element)) _output) (== (`.MaskRadius_10_440B430A4343FB7EE594AFABFE1B9FD7` (break `/Game/DataTables/Masking/S_NatureMask` _array_element)) _output_2)))
          (bind _output_3 (`self.GetMaskCenterArray` (`/Game/Blueprints/GM_Solar.NatureIndex` (`self.GameMode`))))
          (`KismetMaterialLibrary.SetVectorParameterValue` "/Game/VFX/Materials/MPC_MaskingNature.MPC_MaskingNature" _output_3 _returnvalue)
          (`Timeline|GrowRadiusAfter1` :!via `PlayFromStart`
            (:`Update`
              (`self.GrowMaskRadius`))
            (:`Finished`
              (set `self.IsInteractable` false)
              (`ActorComponent.K2_DestroyComponent` (`self.DialogueIndicator`))
              (bind _output_4 (`self.GetMaskCenterArray` _natureindex_2))
              (bind _output_5 (`self.GetMaskRadiusArray` _natureindex_2))
              (`KismetArrayLibrary.Array_Add` (`/Game/Blueprints/GM_Solar.NatureSphereMasks` _gamemode_2) (make `/Game/DataTables/Masking/S_NatureMask` (`KismetSystemLibrary.GetDisplayName` self) _output_4 _output_5 _returnvalue))
              (`/Game/Blueprints/GM_Solar.IncrementNatureIndex` _gamemode_2)
              (`/Game/Blueprints/GM_Solar.UpdateNatureData` _gamemode_2)
              (break))))
        (else
          (`KismetMaterialLibrary.SetVectorParameterValue` "/Game/VFX/Materials/MPC_MaskingNature.MPC_MaskingNature" "MaskCenter" _returnvalue)
          (`|ExecutionSequence`
            (:`then_0`
              (`Timeline|GrowRadius1` :!via `PlayFromStart`
                (:`Update`
                  (`self.GrowNatureFirstTime`))))
            (:`then_1`
              (set `self.IsInteractable` false)
              (`ActorComponent.K2_DestroyComponent` (`self.DialogueIndicator`))
              (`KismetArrayLibrary.Array_Set` (`/Game/Blueprints/GM_Solar.NatureSphereMasks` _gamemode_3) 0 (make `/Game/DataTables/Masking/S_NatureMask` (`KismetSystemLibrary.GetDisplayName` self) "MaskCenter" "MaskRadius" (`KismetMathLibrary.Conv_VectorToLinearColor` (`SceneComponent.K2_GetComponentLocation` (`self.SM_wood_box_01`)))))
              (`/Game/Blueprints/GM_Solar.UpdateNatureData` _gamemode_3)
              (goto _label :!via `Break`)))))))
  (set `self.CurrentRadius` 0.0))

(event `SavedNature`
  ; Increase the radius of the sphere mask so that the second texture takes over and the static mesh changes.
  (for (_array_element _array_index) (`/Game/Blueprints/GM_Solar.NatureSphereMasks` (`self.GameMode`))
    (if (`KismetStringLibrary.EqualEqual_StrStr` (break `/Game/DataTables/Masking/S_NatureMask` _array_element) (`KismetSystemLibrary.GetDisplayName` self))
      (bind _output_get (set `self.SphereMaskIndex` _array_index))
      (bind _output (`self.GetMaskCenterArray` _output_get))
      (`KismetMaterialLibrary.SetVectorParameterValue` "/Game/VFX/Materials/MPC_MaskingNature.MPC_MaskingNature" _output (`KismetMathLibrary.Conv_VectorToLinearColor` (`SceneComponent.K2_GetComponentLocation` (`self.SM_wood_box_01`))))
      (`Timeline|Timeline` :!via `PlayFromStart`
        (:`Update`
          (`self.ReGrowNature`))
        (:`Finished`
          (set `self.IsInteractable` false)
          (`ActorComponent.K2_DestroyComponent` (`self.DialogueIndicator`))
          (`StaticMeshComponent.SetStaticMesh` (`self.SM_wood_box_01`) "/Game/Maps/StylizedProvencal/Meshes/SM_GrassField_01_a.SM_GrassField_01_a")
          (break)))))
  (set `self.CurrentRadius` 0.0))

(event `OnNotEnough_Event`
  (bind (_returnvalue_x _returnvalue_y) (`KismetMathLibrary.BreakVector2D` (`WidgetComponent.GetDrawSize` (`self.Widget`))))
  (bind _sizebox_37 (`/Game/Blueprints/QuickTimeEvents/QTE_HUD2.SizeBox_37` (`self.QTEWidgetRef2`)))
  ; QTE Logic
  (if (and (== (stale `self.QTEGameStart` ActorTarget) (`GameplayStatics.GetPlayerCharacter` 0)) (not (`self.IsActive`))) :!label _label_2
    (add `self.OnNotEnough` (delegate `OnNotEnough_Event`))
    (bind _returnvalue (`|CreateWidget` "/Game/Blueprints/QuickTimeEvents/QTE_HUD2.QTE_HUD2_C" null (`KismetArrayLibrary.Array_Random` (`|MakeArray` "NewEnumerator0" "NewEnumerator1" "NewEnumerator2" "NewEnumerator3" :!type "/Game/Blueprints/QuickTimeEvents/E_QuickTimeInputs Enum")) (`self.TimeToReact`)))
    (`WidgetComponent.SetWidget` (`self.Widget`) _returnvalue)
    (bind _output_get (set `self.QTEWidgetRef2` _returnvalue))
    (add `/Game/Blueprints/QuickTimeEvents/QTE_HUD2.FinishedQTE` _output_get (`|CreateDelegate` :!event `FinishedQTE_Event`))
    (set `self.IsActive` true)
    (`SizeBox.SetHeightOverride` _sizebox_37 _returnvalue_y)
    (`SizeBox.SetWidthOverride` _sizebox_37 _returnvalue_x)))

(event `self.QTEGameStart`
  (params (ActorTarget :type "Actor Object Reference"))
  ; QTE Logic
  (goto _label_2))

(event `FinishedQTE_Event`
  (params (Success :type Boolean))
  (bind _playerinstigates (`self.PlayerInstigates`))
  ; QTE Logic By Nifty
  (set `self.IsActive` false)
  (clear `/Game/Blueprints/QuickTimeEvents/QTE_HUD2.FinishedQTE` (`self.QTEWidgetRef2`))
  (`WidgetComponent.SetWidget` (`self.Widget`) null)
  (set `self.QTEWidgetRef2` null)
  (if Success
    (`/Engine/EditorBlueprintResources/StandardMacros.IncrementInt` (`self.SuccessCounter`)
      (:`  `
        (if (== (`self.SuccessCounter`) 3)
          (`self.RevealNature`)
          (set `/Game/Blueprints/Characters/BP_Character_Base.IsInteractionLocked` true (`self.PlayerInstigates`))
          (`WidgetComponent.SetWidget` (`self.Widget`) null)
          (set `self.SuccessCounter` 0)
          (remove `self.OnNotEnough` (`|CreateDelegate` :!event `OnNotEnough_Event`))
          (`self.EnableInput` _playerinstigates (`GameplayStatics.GetPlayerController` 0))
          (`KismetSystemLibrary.Delay` 0.2)
          (`self.Start Character Interaction` _playerinstigates)
          (`self.StartInteraction` _playerinstigates)
          (`self.ShowDialogueLine`)
          (`self.FinishInteraction`)
          (`FMODBlueprintStatics.PlayEvent2D` "/Game/FMOD/Events/SFX/SFX_CorrectAnswer.SFX_CorrectAnswer")
          (else
            (`self.OnNotEnough`)))))
    (else
      (`WidgetComponent.SetWidget` (`self.Widget`) null)
      (`self.EnableInput` (`self.PlayerInstigates`) (`GameplayStatics.GetPlayerController` 0))
      (`self.FinishInteraction`)
      (`FMODBlueprintStatics.PlayEvent2D` "/Game/FMOD/Events/SFX/SFX_IncorrectAnswer.SFX_IncorrectAnswer"))))

(fn `EndInteraction`
  (set `self.IsInteractionLocked` false))

(fn `GetItemInfo`
  (returns (CurrentInventory :type "Array of /Game/DataTables/Inventory/S_ItemProperties Structure"))
  (return (`/Game/Blueprints/GM_Solar.Items` (`self.GameMode`))))

(fn `GetMaskCenterArray`
  (params (Index :type Integer))
  (returns (Output :type Name))
  (set `self.CenterIndex` Index)
  (return (`|GetArrayItem` (`self.MaskingCenterArray`) Index)))

(fn `GetMaskRadiusArray`
  (params (Index :type Integer))
  (returns (Output :type Name))
  (set `self.RadiusIndex` Index)
  (return (`|GetArrayItem` (`self.MaskingRadiusArray`) Index)))

(fn `GetSmallPile`
  (returns (SmallPileArray :type "Array of /Game/DataTables/Inventory/S_ItemProperties Structure"))
  (bind _asbp_small_pile (cast `/Game/Blueprints/Props/BP_SmallPile` self))
  (return (`/Game/Blueprints/Props/BP_SmallPile.ItemArray` _asbp_small_pile)))

(fn `GrowMaskRadius`
  (bind _returnvalue (`KismetMathLibrary.FInterpTo` (`self.CurrentRadius`) 400.0 (`self.Delta Seconds`) 5.0))
  (bind _output_propsname (break `/Game/DataTables/Masking/S_NatureMask` (`|GetArrayItem` (`/Game/Blueprints/GM_Solar.NatureSphereMasks` (`self.GameMode`)))))
  (if (`KismetStringLibrary.EqualEqual_StrStr` _output_propsname)
    (`KismetMaterialLibrary.SetScalarParameterValue` "/Game/VFX/Materials/MPC_MaskingNature.MPC_MaskingNature" "MaskRadius" _returnvalue)
    (else
      (bind _output (`self.GetMaskRadiusArray` (`/Game/Blueprints/GM_Solar.NatureIndex` (`self.GameMode`))))
      (`KismetMaterialLibrary.SetScalarParameterValue` "/Game/VFX/Materials/MPC_MaskingNature.MPC_MaskingNature" _output _returnvalue)))
  (set `self.CurrentRadius` _returnvalue)
  (return))

(fn `GrowNatureFirstTime`
  (bind _returnvalue (`KismetMathLibrary.FInterpTo` (`self.CurrentRadius`) 400.0 (`self.Delta Seconds`) 5.0))
  (`KismetMaterialLibrary.SetScalarParameterValue` "/Game/VFX/Materials/MPC_MaskingNature.MPC_MaskingNature" "MaskRadius" _returnvalue)
  (set `self.CurrentRadius` _returnvalue)
  (return))

(fn `HideDialogue`
  (`self.EndInteraction`)
  (`/Game/UI/Widgets/WBP_SpeechBubble.HideDialogue` (`/Game/UI/Widgets/WBP_HUD.WBP_SpeechBubble` (`/Game/Blueprints/GM_Solar.HUDWidget` (`self.GameMode`)))))

(fn `QTEGameFinished`
  (returns (Success :type Boolean))
  (return false))

(fn `ReGrowNature`
  (bind _returnvalue (`KismetMathLibrary.FInterpTo` (`self.CurrentRadius`) 400.0 (`self.Delta Seconds`) 5.0))
  (bind _output (`self.GetMaskRadiusArray` (`self.SphereMaskIndex`)))
  (`KismetMaterialLibrary.SetScalarParameterValue` "/Game/VFX/Materials/MPC_MaskingNature.MPC_MaskingNature" _output _returnvalue)
  (set `self.CurrentRadius` _returnvalue)
  (return))

(fn `ShowDialogueLine`
  (bind _returnvalue (`|GetDataTableRow` "/Game/DataTables/Dialogue/DT_Dialogue.DT_Dialogue" (`self.Current Row Name`))
    (:`then`
      (bind (_dialoguetext _nextrow) (break `/Game/DataTables/Dialogue/S_DialogueData` _returnvalue))
      (`/Game/UI/Widgets/WBP_HUD.ShowDialogue` (`/Game/Blueprints/GM_Solar.HUDWidget` (`self.GameMode`)) self (`self.Name`) _dialoguetext)
      (set `self.Next Row` _nextrow)
      (return))))

(fn `ShowNextLine`
  (returns (HasNextLine :type Boolean))
  (if (`KismetStringLibrary.IsEmpty` (`self.Next Row`))
    (set `self.Current Row Name` (`self.Reset Row Name`))
    (return false)
    (else
      (set `self.Current Row Name` (`KismetStringLibrary.Conv_StringToName` (`self.Next Row`)))
      (`self.ShowDialogueLine`)
      (`GameplayStatics.PlaySound2D` "/Game/Sounds/S_Dialogue_Cue.S_Dialogue_Cue" 1.0 1.0 0.0 null null)
      (return true))))

(fn `Start Character Interaction`
  (params (`Player Character` :type "Actor Object Reference"))
  (if (`self.IsInteractable`)
    (bind _asbp_player (cast `/Game/Blueprints/Characters/BP_Player` `Player Character`))
    (`/Game/Blueprints/Characters/BP_Character_Base.StartInteraction` _asbp_player (`self.GetParentActor` _asbp_player))))

(fn `StartInteraction`
  (params (InteractInstigator :type "Actor Object Reference"))
  (if (`self.IsInteractable`)
    (set `self.IsInteractionLocked` true)
    (`GameplayStatics.PlaySound2D` "/Game/Sounds/S_Dialogue_Cue.S_Dialogue_Cue" 0.1 1.0 0.0 null null)))

(fn `UserConstructionScript`)