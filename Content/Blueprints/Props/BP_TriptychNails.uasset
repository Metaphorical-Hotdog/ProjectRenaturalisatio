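; Interactable triptych nails prop that gives its item to the player's inventory and destroys itself at BeginPlay if the player already has nails.
; At BeginPlay it looks up a row name and copies that DTItems row into its item array.
; On interaction it merges the item into a matching stack in the GameMode's inventory, capped at 64, or fills an empty slot, then reloads the inventory.
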(event `self.ReceiveBeginPlay`
  (`parent.ReceiveBeginPlay`)
  (for _index (range 1)
    (bind _rowname (`self.GetItemNameFromArray` _index))
    (`self.SetItemInArray` _rowname _index)
    (bind _asbp_player (cast `/Game/Blueprints/Characters/BP_Player` (`GameplayStatics.GetPlayerCharacter` 0)))
    (if (`/Game/Blueprints/Characters/BP_Player.HasNails` _asbp_player)
      (`self.K2_DestroyActor`))))

(fn `AddItemToInventory`
  (bind _gamemode (`self.GameMode`))
  (bind _gamemode_2 (`self.GameMode`))
  (for (_ _array_index) (`self.ItemArray`)
    (for (_array_element _array_index_2) (`/Game/Blueprints/GM_Solar.Items` (`self.GameMode`))
      (bind (_item_name _amount _stackable) (`self.GetInventoryLoop` _array_index))
      (set `self.PreviousItemName` "")
      (set `self.InventoryArrayIndex` _array_index_2)
      (bind (_itemname _amount_2) (break `/Game/DataTables/Inventory/S_ItemProperties` _array_element))
      (bind _returnvalue (+ _amount _amount_2))
      (if (and (`KismetStringLibrary.EqualEqual_StrStr` _item_name _itemname) _stackable (<= _returnvalue 64))
        (bind (_item_name_2 _amount_3 _stackable_2 _output) (`self.GetInventoryLoop` (`self.Index`)))
        (`KismetArrayLibrary.Array_Set` (`/Game/Blueprints/GM_Solar.Items` _gamemode_2) (`self.InventoryArrayIndex`) (make `/Game/DataTables/Inventory/S_ItemProperties` (break `/Game/DataTables/Inventory/S_ItemProperties` _output) _returnvalue (`.Stackable_23_FA37C4344C9818053EE4659886A759EE` (break `/Game/DataTables/Inventory/S_ItemProperties` _output)) (`.Category_6_A275009B4E4C9E9671E746B0441E09FB` (break `/Game/DataTables/Inventory/S_ItemProperties` _output)) (`.PileSize_5_F3F9635649797D8E07AC34B424E0E089` (break `/Game/DataTables/Inventory/S_ItemProperties` _output)) (`.Image_20_3F6DE9654F99211A289073868539B0CD` (break `/Game/DataTables/Inventory/S_ItemProperties` _output))))
        (set `self.InventoryArrayIndex` 0)
        (`/Game/Blueprints/GM_Solar.UpdateInventoryData` _gamemode_2)
        (break)
        (elif (<= _amount_2 0)
          (bind (_item_name_3 _amount_4 _stackable_3 _output_2) (`self.GetInventoryLoop` (`self.Index`)))
          (if (not (`KismetStringLibrary.EqualEqual_StrStr` (`self.PreviousItemName`) _item_name_3))
            (`KismetArrayLibrary.Array_Set` (`/Game/Blueprints/GM_Solar.Items` _gamemode) (`self.InventoryArrayIndex`) _output_2)
            (`/Game/Blueprints/GM_Solar.UpdateInventoryData` _gamemode)
            (`/Game/Blueprints/GM_Solar.UpdateInventoryData` _gamemode)
            (set `self.InventoryArrayIndex` 0)
            (break)))))))

(fn `GetInventory`
  (returns (Inventory :type "Array of /Game/DataTables/Inventory/S_ItemProperties Structure"))
  (return (`/Game/Blueprints/GM_Solar.Items` (`self.GameMode`))))

(fn `GetInventoryLoop`
  (params (Index :type Integer))
  (returns (`Item Name` :type String) (Amount :type Integer) (Stackable :type Boolean) (Output :type "/Game/DataTables/Inventory/S_ItemProperties Structure (by ref)"))
  (bind _itemarray (`self.ItemArray`))
  (bind (_output_itemname _output_amount _output_stackable) (break `/Game/DataTables/Inventory/S_ItemProperties` (`|GetArrayItem` _itemarray Index)))
  (set `self.Index` Index)
  (return _output_itemname _output_amount _output_stackable (`|GetArrayItem` _itemarray Index)))

(fn `GetInventoryWidget`
  (returns (WBP_Inventory :type "/Game/UI/Widgets/WBP_Inventory Object Reference"))
  (return (`/Game/UI/Widgets/WBP_HUD.WBP_Inventory` (`/Game/Blueprints/GM_Solar.HUDWidget` (`self.GameMode`)))))

(fn `GetItemNameFromArray`
  (params (CurrentIndex :type Integer))
  (returns (RowName :type Name))
  (set `self.CurrentIndex` CurrentIndex)
  (return (`|GetArrayItem` (`self.TableRowName`) (`KismetMathLibrary.RandomInteger` 1))))

(fn `GetItemProperties`
  (returns (ItemProperties :type "/Game/DataTables/Inventory/S_ItemProperties Structure"))
  (for _array_element (`self.ItemArray`)
    (return _array_element)))

(fn `SetItemInArray`
  (params (RowName :type Name) (Index :type Integer))
  (bind _itemarray (`self.ItemArray`))
  (bind _returnvalue (`|GetDataTableRow` (`self.DTItems`) RowName)
    (:`then`
      (bind _returnvalue_2 (`KismetArrayLibrary.Array_Add` _itemarray _returnvalue))
      (`KismetArrayLibrary.Array_Set` _itemarray _returnvalue_2 _returnvalue))))

(fn `StartInteraction`
  (params (InteractInstigator :type "Actor Object Reference"))
  (`parent.StartInteraction` InteractInstigator)
  (`self.AddItemToInventory`)
  (`/Game/Blueprints/GM_Solar.LoadInventory` (`self.GameMode`)))

(fn `UserConstructionScript`
  (`parent.UserConstructionScript`))