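; Player character with a sprite, handling Enhanced Input movement, interaction and inventory toggling, plus K/F test keys.
; Interact messages the first overlapping actor, then advances or instantly reveals dialogue in the HUD speech bubble; movement stops while interaction is locked.
; Each tick restores cached materials, sphere-traces from camera toward sprite and swaps blockers to a transparent occlusion material.
; Tick also feeds player position to MPC_Masking; audio listener follows the sprite.
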(event `self.ReceiveBeginPlay`
  ;[1 1 1] Intializes the controller to be casted to PlayerController, and the Input player Subsystem, adding the IMC to Mapping Context.
  (`parent.ReceiveBeginPlay`)
  (`|ExecutionSequence`
    (:`then_0`
      (bind _asplayer_controller (cast `PlayerController` (`self.GetController`)))
      (`EnhancedInputSubsystemInterface.AddMappingContext` (pcsubsystem `EnhancedInputLocalPlayerSubsystem` _asplayer_controller) "/Game/Input/IMC_Solar.IMC_Solar" 0 (struct)))
    (:`then_1`
      (`PlayerController.SetAudioListenerOverride` (`GameplayStatics.GetPlayerController` 0) (`self.Sprite`) (0.0 0.0 0.0) (struct :`Yaw` 270.0)))))

(event `EnhancedInput|/Game/Input/Actions/IA_Move`
  (params (ActionValue :type "Vector2D Structure") (ElapsedSeconds :type "Float (double-precision)") (TriggeredSeconds :type "Float (double-precision)") (InputAction :type "InputAction Object Reference" :default "/Game/Input/Actions/IA_Move.IA_Move"))
  (bind (_x _y) (`KismetMathLibrary.BreakVector2D` ActionValue))
  ;[1 1 1] Set up the Event for IA_Move and add the movement input for both axis X and Y.
  (:`Triggered`
    (if (not (`self.IsInteractionLocked`))
      (`self.AddMovementInput` (1.0 0.0 0.0) _x)
      (`self.AddMovementInput` (0.0 1.0 0.0) _y))))

(event `EnhancedInput|/Game/Input/Actions/IA_Interact`
  (params (ActionValue :type Boolean) (ElapsedSeconds :type "Float (double-precision)") (TriggeredSeconds :type "Float (double-precision)") (InputAction :type "InputAction Object Reference" :default "/Game/Input/Actions/IA_Interact.IA_Interact"))
  ;[1 1 1] Loop over everything when we press the interact button.
  (:`Started`
    (if (`self.IsInteractionLocked`)
      ;;[1 1 1] If the letters are done being revealed on the bubble, then we can close the bubble.
      (if (`/Game/UI/Widgets/WBP_SpeechBubble.FinishedRevealing` (`self.GetSpeechBubble`))
        (bind _lastinteracted (`self.LastInteracted`)
          (:`then`
            (bind _hasnextline (message `/Game/Blueprints/Interfaces/BPI_Interactable.ShowNextLine` _lastinteracted))
            (if (not _hasnextline)
              ;;[1 1 1] Ends the interaction and finishes it if is interaction locked is set to true.
              (`self.EndInteraction`)
              (bind _lastinteracted_2 (`self.LastInteracted`)
                (:`then`
                  (message `/Game/Blueprints/Interfaces/BPI_Interactable.FinishInteraction` _lastinteracted_2)
                  (`/Game/UI/Widgets/WBP_SpeechBubble.HideDialogue` (`self.GetSpeechBubble`)))
                (:`else`))))
          (:`else`))
        (else
          (`/Game/UI/Widgets/WBP_SpeechBubble.InstantReveal` (`self.GetSpeechBubble`))))
      (else
        (for _array_element (`PrimitiveComponent.GetOverlappingActors` (`self.InteractionCheck`) null)
          (if (!= _array_element self)
            (message `/Game/Blueprints/Interfaces/BPI_Interactable.Interact` _array_element self)
            (set `self.LastInteracted` _array_element)
            (break)))))))

(event `EnhancedInput|/Game/Input/Actions/IA_Inventory`
  (params (ActionValue :type Boolean) (ElapsedSeconds :type "Float (double-precision)") (TriggeredSeconds :type "Float (double-precision)") (InputAction :type "InputAction Object Reference" :default "/Game/Input/Actions/IA_Inventory.IA_Inventory"))
  (bind _wbp_inventory (`self.GetInventory`))
  ;[1 1 1] Opening up Inventory action
  (:`Started`
    (if (`self.IsInventoryOpen`)
      (`/Game/UI/Widgets/WBP_Inventory.HideInventory` _wbp_inventory)
      (set `self.IsInventoryOpen` false)
      (else
        (`/Game/UI/Widgets/WBP_Inventory.ShowInventory` _wbp_inventory)
        (set `self.IsInventoryOpen` true)))))

(event `self.ReceiveTick`
  (params (DeltaSeconds :type "Float (single-precision)"))
  (bind _hiddencomponent (`self.HiddenComponent`))
  (bind _returnvalue (`SceneComponent.K2_GetComponentLocation` (`self.Camera`)))
  (`parent.ReceiveTick` DeltaSeconds)
  ;[0.6146 0 0 0.5] Reset Material to Original
  (for _array_element _hiddencomponent
    (`self.SetMultipleMaterials` (break `/Game/DataTables/S_ComponentMaterial` _array_element) (`.Material_8_D7385A3240317DF582A3E78151077EF5` (break `/Game/DataTables/S_ComponentMaterial` _array_element))))
  (`KismetArrayLibrary.Array_Clear` _hiddencomponent)
  ;[0.5781 0 0 0.5] Detech Obstructing Objects
  (bind _outhits (`KismetSystemLibrary.SphereTraceMulti` :`Start` _returnvalue :`End` (`KismetMathLibrary.VLerp` _returnvalue (`KismetSystemLibrary.GetComponentBounds` (`self.Sprite`)) (`self.Alpha`)) :`Radius` 25.0 :`TraceChannel` "TraceTypeQuery1" :`DrawDebugType` "ForDuration"))
  (for _array_element_2 _outhits
    (bind (_bblockinghit _binitialoverlap _time _distance _location _impactpoint _normal _impactnormal _physmat _hitactor _hitcomponent) (`GameplayStatics.BreakHitResult` _array_element_2))
    ;[0.7708 0 0 0.5] Set Custom Material
    (bind _materiallist (`self.GetMultipleMaterials` _hitcomponent))
    (`KismetArrayLibrary.Array_Add` (`self.HiddenComponent`) (make `/Game/DataTables/S_ComponentMaterial` _hitcomponent _materiallist))
    (`self.ClearAllMaterials` _hitcomponent)
    (`PrimitiveComponent.SetMaterial` _hitcomponent 0 "/Game/VFX/Materials/M_TransparentOcclusion.M_TransparentOcclusion"))
  ;[1 1 1] This is informing the Material Parameter Location the location of the player. This is for Masking
  (`KismetMaterialLibrary.SetVectorParameterValue` "/Game/VFX/Materials/MPC_Masking.MPC_Masking" "PlayPosition" (`KismetMathLibrary.Conv_VectorToLinearColor` (`self.K2_GetActorLocation`))))

(event `Key|K`
  (params (Key :type "Key Structure"))
  (:`Pressed`
    (`GameplayStatics.OpenLevel` "LEVEL_TestInventory")))

(event `Key|F`
  (params (Key :type "Key Structure"))
  (:`Pressed`
    (`/Game/UI/Widgets/WBP_Inventory.CheckInventory` (`self.GetInventory`))))

(fn `ClearAllMaterials`
  (params (Component :type "PrimitiveComponent Object Reference"))
  (for _index (range (`PrimitiveComponent.GetNumMaterials` Component))
    (`PrimitiveComponent.SetMaterial` Component _index null)))

(fn `GetInventory`
  (returns (WBP_Inventory :type "/Game/UI/Widgets/WBP_Inventory Object Reference"))
  (return (`/Game/UI/Widgets/WBP_HUD.WBP_Inventory` (`/Game/Blueprints/GM_Solar.HUDWidget` (`self.GameMode`)))))

(fn `GetMultipleMaterials`
  (params (Component :type "PrimitiveComponent Object Reference"))
  (returns (MaterialList :type "Array of MaterialInterface Object Reference"))
  (bind _materiallist (`self.MaterialList`))
  (for _index (range (`PrimitiveComponent.GetNumMaterials` Component))
    (`KismetArrayLibrary.Array_Add` _materiallist (`PrimitiveComponent.GetMaterial` Component _index)))
  (return _materiallist))

(fn `GetSpeechBubble`
  (returns (WBP_SpeechBubble :type "/Game/UI/Widgets/WBP_SpeechBubble Object Reference"))
  (return (`/Game/UI/Widgets/WBP_HUD.WBP_SpeechBubble` (`/Game/Blueprints/GM_Solar.HUDWidget` (`self.GameMode`)))))

(fn `SetMultipleMaterials`
  (params (Component :type "PrimitiveComponent Object Reference") (`Material List` :type "Array of MaterialInterface Object Reference"))
  (for (_array_element _array_index) `Material List`
    (`PrimitiveComponent.SetMaterial` Component _array_index _array_element)))

(fn `UserConstructionScript`
  (`parent.UserConstructionScript`))