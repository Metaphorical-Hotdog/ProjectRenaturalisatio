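; Base character Blueprint that gives characters interactable, multi-line dialogue.
; Interact locks the interaction, stops movement and sends the current DT_Dialogue row to the Game Mode's HUD, or plays a bleat when no row is set.
; Lines chain through each row's NextRow, returning to the starting row when the chain ends.
; Ending an interaction releases the lock unless the player is cutscene-locked.
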(event `self.ReceiveBeginPlay`
  ;[1 1 1] This is to cast shadows on the Dialogue Widget
  (`PrimitiveComponent.SetCastShadow` (`self.DialogueIndicator`) false)
  (set `self.Reset Row Name` (`self.Current Row Name`))
  ;[1 1 1] This is to set a reference to Game Mode for all Characters
  (bind _asgm_solar (cast `/Game/Blueprints/GM_Solar` (`GameplayStatics.GetGameMode`)))
  (set `self.GameMode` _asgm_solar))

(event `/Game/Blueprints/Interfaces/BPI_Interactable.Interact`
  (params (Instigator :type "/Game/Blueprints/Characters/BP_Character_Base Object Reference"))
  ;[1 1 1] Display Dialogue through Interface
  (if (!= (`self.Current Row Name`) "None")
    (`self.StartInteraction` Instigator null)
    (`self.StartInteraction` Instigator)
    (`self.ShowDialogueLine`)
    (else
      (`FMODBlueprintStatics.PlayEvent2D` "/Game/FMOD/Events/SFX/SFX_PandaBleats.SFX_PandaBleats"))))

(event `/Game/Blueprints/Interfaces/BPI_Interactable.FinishInteraction`
  ;[1 1 1] Display Dialogue through Interface
  ;;[1 1 1] Ends the interaction, the rest is handled on BP Player
  (`self.EndInteraction`))

(fn `EndInteraction`
  (bind _asbp_player (cast `/Game/Blueprints/Characters/BP_Player` (`GameplayStatics.GetPlayerCharacter` 0)))
  (if (not (`/Game/Blueprints/Characters/BP_Player.IsCutsceneLocked` _asbp_player))
    (set `self.IsInteractionLocked` false)))

(fn `HideDialogue`
  (`self.EndInteraction`)
  (`/Game/UI/Widgets/WBP_SpeechBubble.HideDialogue` (`/Game/UI/Widgets/WBP_HUD.WBP_SpeechBubble` (`/Game/Blueprints/GM_Solar.HUDWidget` (`self.GameMode`)))))

(fn `ShowDialogueLine`
  (bind _returnvalue (`|GetDataTableRow` "/Game/DataTables/Dialogue/DT_Dialogue.DT_Dialogue" (`self.Current Row Name`))
    (:`then`
      (bind (_dialoguetext _nextrow) (break `/Game/DataTables/Dialogue/S_DialogueData` _returnvalue))
      (`/Game/UI/Widgets/WBP_HUD.ShowDialogue` (`/Game/Blueprints/GM_Solar.HUDWidget` (`self.GameMode`)) self (`self.Name`) _dialoguetext)
      (set `self.Next Row` _nextrow)
      (return))))

(fn `ShowNextLine`
  (returns (HasNextLine :type Boolean))
  (if (`KismetStringLibrary.IsEmpty` (`self.Next Row`))
    (set `self.Current Row Name` (`self.Reset Row Name`))
    (return false)
    (else
      (set `self.Current Row Name` (`KismetStringLibrary.Conv_StringToName` (`self.Next Row`)))
      (`self.ShowDialogueLine`)
      (`GameplayStatics.PlaySound2D` "/Game/Sounds/S_Dialogue_Cue.S_Dialogue_Cue" 1.0 1.0 0.0 null null)
      (return true))))

(fn `StartInteraction`
  (params (InteractInstigator :type "Actor Object Reference"))
  (set `self.IsInteractionLocked` true)
  (`MovementComponent.StopMovementImmediately` (`self.CharacterMovement`))
  (`GameplayStatics.PlaySound2D` "/Game/Sounds/S_Dialogue_Cue.S_Dialogue_Cue" 0.1 1.0 0.0 null null))

(fn `UserConstructionScript`)