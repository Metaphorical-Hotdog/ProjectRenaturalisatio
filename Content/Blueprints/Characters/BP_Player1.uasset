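; Player character Blueprint with a sprite, handling Enhanced Input movement, inventory, dialogue and puzzle pickups.
; Interact messages overlapping actors, then advances or instantly reveals HUD speech-bubble lines, with a branch for cutscenes.
; Opening the inventory stops walking, switches to UI input and eases the camera via timeline, with CloseInventory easing it back.
; It also carries BP_Box objects, counts scrap and feeds its location to MPC_Masking each tick.
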(event `self.ReceivePossessed`
  (params (NewController :type "Controller Object Reference"))
  ;[1 1 1] Intializes the controller to be casted to PlayerController, and the Input player Subsystem, adding the IMC to Mapping Context.
  (bind _asplayer_controller (cast `PlayerController` (`self.GetController`) :!label _label))
  (`EnhancedInputSubsystemInterface.AddMappingContext` (pcsubsystem `EnhancedInputLocalPlayerSubsystem` _asplayer_controller) "/Game/Input/IMC_Solar.IMC_Solar" 0 (struct)))

(event `self.ReceiveBeginPlay`
  ;[1 1 1] Intializes the controller to be casted to PlayerController, and the Input player Subsystem, adding the IMC to Mapping Context.
  (`parent.ReceiveBeginPlay`)
  (`|ExecutionSequence`
    (:`then_0`
      (goto _label))
    (:`then_1`
      (`PlayerController.SetAudioListenerOverride` (`GameplayStatics.GetPlayerController` 0) (`self.Sprite`) (0.0 0.0 0.0) (struct :`Yaw` 270.0)))))

(event `EnhancedInput|/Game/Input/Actions/IA_Inventory`
  (params (ActionValue :type Boolean) (ElapsedSeconds :type "Float (double-precision)") (TriggeredSeconds :type "Float (double-precision)") (InputAction :type "InputAction Object Reference" :default "/Game/Input/Actions/IA_Inventory.IA_Inventory"))
  ;[1 1 1] Opening up Inventory/Crafting action
  (:`Started`
    (if (not (`self.IsInventoryOpen`))
      (set `CharacterMovementComponent.MaxWalkSpeed` 0.0 (`self.CharacterMovement`))
      (`/Game/UI/Widgets/WBP_HUD.ShowMenu` (`self.GetIMenu`))
      (`WidgetBlueprintLibrary.SetInputMode_UIOnlyEx` (`GameplayStatics.GetPlayerController` 0) (`/Game/Blueprints/GM_Solar.HUDWidget` (`self.GameMode`)))
      (set `self.IsInventoryOpen` true)
      (set `PlayerController.bShowMouseCursor` true (`GameplayStatics.GetPlayerController` 0))
      (bind (_direction _inventorytrack) (`Timeline|CameraTransformToInventory` :!via `PlayFromStart`)
        (:`Update`
          (`self.TransformCameraToInventory` _inventorytrack)
          (`self.K2_SetActorRotation` self (struct :`Yaw` 180.0) false))))))

(event `EnhancedInput|/Game/Input/Actions/IA_Move`
  (params (ActionValue :type "Vector2D Structure") (ElapsedSeconds :type "Float (double-precision)") (TriggeredSeconds :type "Float (double-precision)") (InputAction :type "InputAction Object Reference" :default "/Game/Input/Actions/IA_Move.IA_Move"))
  (bind (_x _y) (`KismetMathLibrary.BreakVector2D` ActionValue))
  ;[1 1 1] Set up the Event for IA_Move and add the movement input for both axis X and Y.
  (:`Triggered`
    (if (not (`self.IsInteractionLocked`))
      (`self.AddMovementInput` (1.0 0.0 0.0) _x)
      (`self.AddMovementInput` (0.0 1.0 0.0) _y))))

(event `CloseInventory`
  ;[0 1 0.1977 0.5] Close Inventory when its opened.
  (bind (_direction _newtrack_1) (`Timeline|CloseInventoryTimeline` :!via `PlayFromStart`)
    (:`Update`
      (`self.TransformCameraToDefault` _newtrack_1))))

(event `EnhancedInput|/Game/Input/Actions/IA_Interact`
  (params (ActionValue :type Boolean) (ElapsedSeconds :type "Float (double-precision)") (TriggeredSeconds :type "Float (double-precision)") (InputAction :type "InputAction Object Reference" :default "/Game/Input/Actions/IA_Interact.IA_Interact"))
  ;[0 1 0.1356] Loop over everything when we press the interact button.
  (:`Started`
    (if (`self.IsInteractionLocked`)
      ;;[1 1 1] If the letters are done being revealed on the bubble, then we can close the bubble.
      (if (`self.IsCutsceneLocked`)
        (if (not (`MovieSceneSequencePlayer.IsPlaying` (`self.SequencerPlayer`)))
          (`KismetSystemLibrary.PrintString` "Play Cutscene")
          (`self.OnPlayCutscene`)
          (if (`/Game/UI/Widgets/WBP_SpeechBubble.FinishedRevealing` (`self.GetSpeechBubble`)) :!label _label_2
            (bind _lastinteracted (`self.LastInteracted`)
              (:`then`
                (bind _hasnextline (message `/Game/Blueprints/Interfaces/BPI_Interactable.ShowNextLine` _lastinteracted))
                (if (not _hasnextline)
                  ;;[1 1 1] Ends the interaction and finishes it if is interaction locked is set to true.
                  (`self.EndInteraction`)
                  (bind _lastinteracted_2 (`self.LastInteracted`)
                    (:`then`
                      (message `/Game/Blueprints/Interfaces/BPI_Interactable.FinishInteraction` _lastinteracted_2)
                      (`/Game/UI/Widgets/WBP_SpeechBubble.HideDialogue` (`self.GetSpeechBubble`)))
                    (:`else`))))
              (:`else`))
            (else
              (`/Game/UI/Widgets/WBP_SpeechBubble.InstantReveal` (`self.GetSpeechBubble`)))))
        (else
          (goto _label_2)))
      (else
        (for _array_element (`PrimitiveComponent.GetOverlappingActors` (`self.InteractionCheck`) null)
          (if (!= _array_element self)
            (message `/Game/Blueprints/Interfaces/BPI_Interactable.Interact` _array_element self)
            (set `self.LastInteracted` _array_element)
            (break)))))))

(event `Key|K`
  (params (Key :type "Key Structure"))
  ; Test Inventory by changing levels
  (:`Pressed`
    (`GameplayStatics.OpenLevel` "LEVEL_TestInventory")))

(event `self.ReceiveTick`
  (params (DeltaSeconds :type "Float (single-precision)"))
  (set `self.Delta Seconds` DeltaSeconds)
  (`parent.ReceiveTick` DeltaSeconds)
  ;[1 1 1] This is informing the Material Parameter Location the location of the player. This is for Masking
  (`KismetMaterialLibrary.SetVectorParameterValue` "/Game/VFX/Materials/MPC_Masking.MPC_Masking" "PlayPosition" (`KismetMathLibrary.Conv_VectorToLinearColor` (`self.K2_GetActorLocation`)))
  (add `self.OnLeavingMapRight` (delegate `LeaveAreaRight`)))

(event `LeaveAreaRight`
  (`Timeline|Timeline`
    (:`Update`
      (`self.AddMovementInput` (`KismetMathLibrary.VInterpTo` (`self.K2_GetActorLocation`) (`self.World Direction`) (`self.Delta Seconds`) 5.0)))))

(event `Pickup box`
  (bind _returnvalue (`self.K2_GetActorLocation`))
  ; Puzzle Logic
  (if (not (`self.IsHoldingItem`))
    (bind (_outhit _returnvalue_2) (`KismetSystemLibrary.SphereTraceSingleForObjects` :`Start` _returnvalue :`End` _returnvalue :`Radius` 120.0 :`ObjectTypes` (`|MakeArray` "ObjectTypeQuery4" :!type "EObjectTypeQuery Enum") :`DrawDebugType` "ForDuration"))
    (if _returnvalue_2
      (bind _asbp_box (cast `/Game/Blueprints/Puzzles/PuzzleRoom2/BP_Box` (`.HitActor` (`GameplayStatics.BreakHitResult` _outhit))))
      (`self.K2_AttachToComponent` _asbp_box (`self.PhysicsConstraint`) "None" "SnapToTarget" "SnapToTarget" "KeepWorld" true)
      (set `self.IsHoldingItem` true)
      (`PrimitiveComponent.SetSimulatePhysics` (`/Game/Blueprints/Puzzles/PuzzleRoom2/BP_Box.Cube` _asbp_box) false))))

(event `Drop Box`
  ; Puzzle Logic
  (if (`self.IsHoldingItem`)
    (`self.K2_DetachFromActor` (stale `Pickup box` _asbp_box) "KeepWorld" "KeepWorld" "KeepWorld")
    (set `self.IsHoldingItem` false)
    (`PrimitiveComponent.SetSimulatePhysics` (`/Game/Blueprints/Puzzles/PuzzleRoom2/BP_Box.Cube` (stale `Pickup box` _asbp_box)) true)))

(event `Add Scrap`
  (`/Engine/EditorBlueprintResources/StandardMacros.IncrementInt` (`self.Scrap`)
    (:`  `
      (if (>= (`self.Scrap`) 3)
        (set `self.HasScrap` true)
        (`KismetSystemLibrary.PrintString` "SCRAP ADDED")))))

(event `InteractCutscene`
  (if (`self.IsInteractionLocked`)
    (if (`/Game/UI/Widgets/WBP_SpeechBubble.FinishedRevealing` (`self.GetSpeechBubble`))
      (bind _lastinteracted (`self.LastInteracted`)
        (:`then`
          (bind _hasnextline (message `/Game/Blueprints/Interfaces/BPI_Interactable.ShowNextLine` _lastinteracted))
          (if (not _hasnextline)
            ;[1 1 1] Ends the interaction and finishes it if is interaction locked is set to true.
            (`self.EndInteraction`)
            (bind _lastinteracted_2 (`self.LastInteracted`)
              (:`then`
                (message `/Game/Blueprints/Interfaces/BPI_Interactable.FinishInteraction` _lastinteracted_2)
                (`/Game/UI/Widgets/WBP_SpeechBubble.HideDialogue` (`self.GetSpeechBubble`)))
              (:`else`))))
        (:`else`))
      (else
        (`/Game/UI/Widgets/WBP_SpeechBubble.InstantReveal` (`self.GetSpeechBubble`))))
    (else
      (for _array_element (`PrimitiveComponent.GetOverlappingActors` (`self.InteractionCheck`) null)
        (if (!= _array_element self)
          (message `/Game/Blueprints/Interfaces/BPI_Interactable.Interact` _array_element self)
          (set `self.LastInteracted` _array_element)
          (break))))))

(fn `GetIMenu`
  (returns (HUDWidget :type "/Game/UI/Widgets/WBP_HUD Object Reference"))
  (return (`/Game/Blueprints/GM_Solar.HUDWidget` (`self.GameMode`))))

(fn `GetSpeechBubble`
  (returns (WBP_SpeechBubble :type "/Game/UI/Widgets/WBP_SpeechBubble Object Reference"))
  (return (`/Game/UI/Widgets/WBP_HUD.WBP_SpeechBubble` (`/Game/Blueprints/GM_Solar.HUDWidget` (`self.GameMode`)))))

(fn `TransformCameraToDefault`
  (params (DeltaTime :type "Float (single-precision)"))
  (bind _camera (`self.Camera`))
  (`SceneComponent.K2_SetRelativeTransform` _camera (`KismetMathLibrary.TInterpTo` (`SceneComponent.GetRelativeTransform` _camera) (`self.CameraTransform`) DeltaTime 3.0) false false))

(fn `TransformCameraToInventory`
  (params (DeltaTime :type "Float (single-precision)"))
  (bind _camera (`self.Camera`))
  (`SceneComponent.K2_SetRelativeTransform` _camera (`KismetMathLibrary.TInterpTo` (`SceneComponent.GetRelativeTransform` _camera) (`self.InventoryCameraTransform`) DeltaTime 3.0) false false))

(fn `UserConstructionScript`
  (`parent.UserConstructionScript`))