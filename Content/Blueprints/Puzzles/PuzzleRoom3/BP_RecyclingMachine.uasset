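; BP_RecyclingMachine is an interactable puzzle machine in Puzzle Room 3 that grants the player a lens for the projector.
; On Interact, it casts the instigator to BP_Player and requires both the HasScrap and HasButton flags before setting HasLense.
; Each outcome sends objective text through BP_OBJUpdate: place the lens, missing button, or collect scrap.
; ShowNextLine is a stub that always returns false.
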(event `/Game/Blueprints/Interfaces/BPI_Interactable.Interact`
  (params (Instigator :type "/Game/Blueprints/Characters/BP_Character_Base Object Reference"))
  (bind _asbp_player (cast `/Game/Blueprints/Characters/BP_Player` Instigator))
  (if (`/Game/Blueprints/Characters/BP_Player.HasScrap` _asbp_player)
    (if (`/Game/Blueprints/Characters/BP_Player.HasButton` _asbp_player)
      (set `/Game/Blueprints/Characters/BP_Player.HasLense` true _asbp_player)
      (bind _returnvalue (`GameplayStatics.GetActorOfClass` "/Game/Blueprints/Objectives/BP_OBJUpdate.BP_OBJUpdate_C"))
      (`/Game/Blueprints/Objectives/BP_OBJUpdate.New Objective` _returnvalue "Place Lens in Projector")
      (else
        (`/Game/Blueprints/Objectives/BP_OBJUpdate.New Objective` _returnvalue "The Recycler is missing a button...")))
    (else
      (bind _returnvalue_2 (`GameplayStatics.GetActorOfClass` "/Game/Blueprints/Objectives/BP_OBJUpdate.BP_OBJUpdate_C"))
      (`/Game/Blueprints/Objectives/BP_OBJUpdate.New Objective` _returnvalue_2 "Collect Scrap For the Machine "))))

(fn `ShowNextLine`
  (returns (HasNextLine :type Boolean))
  (return false))

(fn `UserConstructionScript`)