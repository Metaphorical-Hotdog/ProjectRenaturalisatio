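; BP_Triptych1 is the first triptych puzzle object, which opens a puzzle UI when the player interacts or chooses it.
; It binds OpenTriptych to the player's OnChoosingFirstTriptych event at BeginPlay and registers itself with the player's GameMode on opening.
; If unsolved, it shows the Triptych_1 widget when the player has paint, otherwise Triptych1NoTool, then switches to UI-only input with a visible cursor.
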(event `self.ReceiveBeginPlay`
  (bind _asbp_player (cast `/Game/Blueprints/Characters/BP_Player` (`GameplayStatics.GetPlayerCharacter` 0)))
  (bind _output_get (set `self.Player Ref` _asbp_player))
  (add `/Game/Blueprints/Characters/BP_Player.OnChoosingFirstTriptych` _output_get (delegate `Open Triptych`))
  (add `/Game/Blueprints/Characters/BP_Player.OnChoosingFirstTriptych` _asbp_player (delegate `Open Triptych`)))

(event `Open Triptych`
  (bind _returnvalue (`GameplayStatics.GetPlayerController` 0))
  (bind _asbp_player (cast `/Game/Blueprints/Characters/BP_Player` (`GameplayStatics.GetPlayerCharacter` 0)))
  (set `/Game/Blueprints/GM_Solar.FirstTriptych` self (`/Game/Blueprints/Characters/BP_Character_Base.GameMode` _asbp_player))
  (if (not (`self.Solved`))
    (if (`/Game/Blueprints/Characters/BP_Player.HasPaint` _asbp_player)
      (bind _returnvalue_2 (`|CreateWidget` "/Game/UI/Widgets/Puzzles/Triptych_1/Triptych_1.Triptych_1_C"))
      (set `/Game/UI/Widgets/Puzzles/Triptych_1/Triptych_1.GameMode` (`self.GameMode`) _returnvalue_2)
      (`UserWidget.AddToViewport` _returnvalue_2 0)
      (else
        (bind _returnvalue_3 (`|CreateWidget` "/Game/UI/Widgets/Puzzles/Triptych_1/Triptych1NoTool.Triptych1NoTool_C"))
        (`UserWidget.AddToViewport` _returnvalue_3 0)))
    (`WidgetBlueprintLibrary.SetInputMode_UIOnlyEx` _returnvalue null)
    (set `PlayerController.bShowMouseCursor` true _returnvalue)))

(event `self.Interact`
  (params (Instigator :type "/Game/Blueprints/Characters/BP_Character_Base Object Reference"))
  (`self.Open Triptych`))

(fn `ShowNextLine`
  (returns (HasNextLine :type Boolean))
  (return false))

(fn `UserConstructionScript`)