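; BP_Triptych2 is an interactable puzzle object for the second triptych, opening its puzzle screen for the player.
; On BeginPlay it binds OpenTriptych to the player's second-triptych choice event; Interact calls it too.
; OpenTriptych registers itself with the GameMode and, while unsolved, shows either the puzzle widget or a no-tool variant depending on whether the player has nails.
; It then switches input to UI-only with a visible cursor.
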(event `self.ReceiveBeginPlay`
  (bind _asbp_player (cast `/Game/Blueprints/Characters/BP_Player` (`GameplayStatics.GetPlayerCharacter` 0)))
  (bind _output_get (set `self.Player Ref` _asbp_player))
  (add `/Game/Blueprints/Characters/BP_Player.OnChoosingSecondTriptych` _output_get (delegate `OpenTriptych`)))

(event `OpenTriptych`
  (bind _returnvalue (`GameplayStatics.GetPlayerController` 0))
  (bind _asbp_player (cast `/Game/Blueprints/Characters/BP_Player` (`GameplayStatics.GetPlayerCharacter` 0)))
  (set `/Game/Blueprints/GM_Solar.SecondTriptych` self (`/Game/Blueprints/Characters/BP_Character_Base.GameMode` _asbp_player))
  (if (not (`self.Solved`))
    (if (`/Game/Blueprints/Characters/BP_Player.HasNails` (`self.Player Ref`))
      (bind _returnvalue_2 (`|CreateWidget` "/Game/UI/Widgets/Puzzles/Triptych_2/Triptych_2.Triptych_2_C"))
      (set `/Game/UI/Widgets/Puzzles/Triptych_2/Triptych_2.GameMode` (`self.GameMode`) _returnvalue_2)
      (`UserWidget.AddToViewport` _returnvalue_2 2)
      (else
        (bind _returnvalue_3 (`|CreateWidget` "/Game/UI/Widgets/Puzzles/Triptych_2/Triptych_2_NoTool.Triptych_2_NoTool_C"))
        (`UserWidget.AddToViewport` _returnvalue_3 2)))
    (`WidgetBlueprintLibrary.SetInputMode_UIOnlyEx` _returnvalue null)
    (set `PlayerController.bShowMouseCursor` true _returnvalue)))

(event `self.Interact`
  (params (Instigator :type "/Game/Blueprints/Characters/BP_Character_Base Object Reference"))
  (`self.OpenTriptych`))

(fn `ShowNextLine`
  (returns (HasNextLine :type Boolean))
  (return false))

(fn `UserConstructionScript`)