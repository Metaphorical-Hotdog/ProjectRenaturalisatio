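; BP_Triptych3 is an interactable electricity-puzzle actor that opens the third triptych UI, either on Interact or when the player's third-triptych event fires.
; It shows the puzzle widget if the player has glue, otherwise a no-tools variant, and switches input to UI-only with a cursor.
; Closing pauses triptych music and resumes overworld music; the puzzle widget is also cached for re-adding on later opens.
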(event `self.ReceiveBeginPlay`
  (bind _asbp_player (cast `/Game/Blueprints/Characters/BP_Player` (`GameplayStatics.GetPlayerCharacter` 0)))
  (bind _output_get (set `self.Player Ref` _asbp_player))
  (add `/Game/Blueprints/Characters/BP_Player.OnChoosingThirdTriptych` _output_get (delegate `OpenTriptych`))
  (`KismetSystemLibrary.Delay` 0.01)
  (bind _asgm_solar (cast `/Game/Blueprints/GM_Solar` (`GameplayStatics.GetGameMode`)))
  (set `self.GameMode` _asgm_solar))

(event `OpenTriptych`
  (bind _returnvalue (`GameplayStatics.GetPlayerController` 0))
  (bind _asbp_player (cast `/Game/Blueprints/Characters/BP_Player` (`GameplayStatics.GetPlayerCharacter` 0)))
  (set `/Game/Blueprints/GM_Solar.ThirdTriptych` self (`/Game/Blueprints/Characters/BP_Character_Base.GameMode` _asbp_player))
  (if (`/Game/Blueprints/Characters/BP_Player.HasGlue` (`self.Player Ref`))
    (if (`self.Triptych3Shown`)
      (`UserWidget.AddToViewport` (`self.Widget`) 2)
      (else
        (bind _returnvalue_2 (`|CreateWidget` "/Game/UI/Widgets/Puzzles/Triptych_3/WBP_Triptych3.WBP_Triptych3_C"))
        (set `/Game/UI/Widgets/Puzzles/Triptych_3/WBP_Triptych3.GameMode` (`self.GameMode`) _returnvalue_2)
        (`UserWidget.AddToViewport` _returnvalue_2 2)
        (`WidgetBlueprintLibrary.SetInputMode_UIOnlyEx` _returnvalue null :!label _label)
        (set `PlayerController.bShowMouseCursor` true _returnvalue)
        (add `/Game/UI/Widgets/Puzzles/Triptych_3/WBP_Triptych3.OnTriptych3Closed` _returnvalue_2 (delegate `HideTriptych`))
        (add `/Game/UI/Widgets/Puzzles/Triptych_3/WBP_Triptych3NoTools.onTriptych3NoToolsClosed` (stale _returnvalue_3) (delegate `HideNoTools`))))
    (else
      (bind _returnvalue_3 (`|CreateWidget` "/Game/UI/Widgets/Puzzles/Triptych_3/WBP_Triptych3NoTools.WBP_Triptych3NoTools_C"))
      (`UserWidget.AddToViewport` _returnvalue_3 2)
      (goto _label))))

(event `HideNoTools`
  (bind _gameinstance (`/Game/Blueprints/GM_Solar.GameInstance` (`self.GameMode`)))
  (`FMODBlueprintStatics.EventInstanceSetPaused` (`/Game/Blueprints/GI_Solar.triptychMusic` _gameinstance) true :!label _label_2)
  (`FMODBlueprintStatics.EventInstanceSetPaused` (`/Game/Blueprints/GI_Solar.OverworldMusic` _gameinstance)))

(event `HideTriptych`
  (set `self.Widget` (stale `OpenTriptych` _returnvalue_2))
  (set `self.Triptych3Shown` true)
  (goto _label_2))

(event `self.Interact`
  (params (Instigator :type "/Game/Blueprints/Characters/BP_Character_Base Object Reference"))
  (`self.OpenTriptych`))

(fn `ShowNextLine`
  (returns (HasNextLine :type Boolean))
  (return false))

(fn `UserConstructionScript`)