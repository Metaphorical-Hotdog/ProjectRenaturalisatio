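; Puzzle room sliding door that moves vertically once enough switches are active.
; Switch activation and deactivation events adjust a counter, which is compared with the required count to set DoorUp.
; The DoorOpening timeline drives the door's relative Z, playing to open and reversing when too few switches are active.
; An overlapping BP_Box halts the timeline, which resumes in the DoorUp direction when the overlap ends.
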(event `Switch Activated`
  (bind _switches_active (`self.Switches Active`))
  (`/Engine/EditorBlueprintResources/StandardMacros.IncrementInt` _switches_active
    (:`  `
      (if (>= _switches_active (`self.Switches Needed`))
        (set `self.Door Up` true)
        (bind (_direction _door_opening) (`Timeline|Door Opening` :!label _label)
          (:`Update`
            (`SceneComponent.K2_SetRelativeLocation` (`self.Door`) (`KismetMathLibrary.MakeVector` 0.0 0.0 _door_opening) false false)))
        (else
          (set `self.Door Up` false)
          (goto _label :!via `Reverse`))))))

(event `Switch Deactivated`
  (bind _switches_active (`self.Switches Active`))
  (`/Engine/EditorBlueprintResources/StandardMacros.DecrementInt` _switches_active
    (:`  `
      (if (>= _switches_active (`self.Switches Needed`))
        (set `self.Door Up` true)
        (else
          (set `self.Door Up` false)
          (goto _label :!via `Reverse`))))))

(event `self.ReceiveActorBeginOverlap`
  (params (OtherActor :type "Actor Object Reference"))
  (cast `/Game/Blueprints/Puzzles/PuzzleRoom2/BP_Box` OtherActor)
  (goto _label :!via `Stop`))

(event `self.ReceiveActorEndOverlap`
  (params (OtherActor :type "Actor Object Reference"))
  (cast `/Game/Blueprints/Puzzles/PuzzleRoom2/BP_Box` OtherActor)
  (if (`self.Door Up`)
    (goto _label)
    (else
      (goto _label :!via `Reverse`))))

(fn `UserConstructionScript`)