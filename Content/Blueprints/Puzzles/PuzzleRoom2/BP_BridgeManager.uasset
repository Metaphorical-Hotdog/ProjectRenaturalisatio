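; BP_BridgeManager is a puzzle manager in PuzzleRoom2 that watches whether three bridge pieces are slotted.
; Every Tick it calls PuzzleCheck, which tests the Slotted flag on Bridge1, Bridge2 and Bridge3 and enters a DoOnce when all are set.
; Nothing follows the DoOnce, so completion has no effect here.
; BeginPlay stores a BP_BridgeSlot in BridgeRef, which the check does not use.
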(event `self.ReceiveBeginPlay`
  (bind _returnvalue (`GameplayStatics.GetActorOfClass` "/Game/Blueprints/Puzzles/PuzzleRoom2/BP_BridgeSlot.BP_BridgeSlot_C"))
  (set `self.BridgeRef` _returnvalue))

(event `self.ReceiveTick`
  (params (DeltaSeconds :type "Float (single-precision)"))
  (`self.Puzzle Check`))

(event `Puzzle Check`
  (if (and (`/Game/Blueprints/Puzzles/PuzzleRoom2/BP_BridgeSlot.Slotted` (`self.Bridge 1`)) (`/Game/Blueprints/Puzzles/PuzzleRoom2/BP_BridgeSlot.Slotted` (`self.Bridge 2`)) (`/Game/Blueprints/Puzzles/PuzzleRoom2/BP_BridgeSlot.Slotted` (`self.Bridge 3`)))
    (`/Engine/EditorBlueprintResources/StandardMacros.DoOnce` false)))

(fn `UserConstructionScript`)