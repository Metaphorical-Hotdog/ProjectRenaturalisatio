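; BP_Box is an interactable box for Puzzle Room 2 that the player repairs with a wrench, then carries.
; Interact requires the player to hold the wrench; the first use marks it repaired, and later uses set a metal material and alternate between pickup and drop through a FlipFlop.
; Pickup and drop are delegated to BP_Player, and destroying the box clears that player's holding-item flag.
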(event `/Game/Blueprints/Interfaces/BPI_Interactable.Interact`
  (params (Instigator :type "/Game/Blueprints/Characters/BP_Character_Base Object Reference"))
  (bind _player_ref_2 (`self.Player ref 2`))
  (bind _asbp_player (cast `/Game/Blueprints/Characters/BP_Player` Instigator))
  (set `self.Player ref 2` _asbp_player)
  (if (`/Game/Blueprints/Characters/BP_Player.HasWrench` _player_ref_2)
    (if (`self.Is Repaired`)
      (`PrimitiveComponent.SetMaterial` (`self.Cube`) 0 "/Game/2DAssets/Environment/Textures/Materials/MI_Metal.MI_Metal")
      (`/Engine/EditorBlueprintResources/StandardMacros.FlipFlop`
        (:`A`
          (`/Game/Blueprints/Characters/BP_Player.Pickup box` _player_ref_2)
          (set `self.Is Held` true))
        (:`B`
          (`/Game/Blueprints/Characters/BP_Player.Drop Box` _player_ref_2)
          (set `self.Is Held` false)))
      (else
        (set `self.Is Repaired` true)))))

(event `self.ReceiveDestroyed`
  (set `/Game/Blueprints/Characters/BP_Player.IsHoldingItem` false (`self.Player ref 2`)))

(fn `ShowNextLine`
  (returns (HasNextLine :type Boolean))
  (return false))

(fn `UserConstructionScript`)