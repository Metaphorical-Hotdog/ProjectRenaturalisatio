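; BP_Box_Fixed is an interactable box in Puzzle Room 2 that the player must repair with a wrench before carrying it.
; Interacting without the wrench shows a "NoWrench" dialogue line; the first interaction with it marks the box repaired and shows "BoxFixed" dialogue.
; Later interactions alternate pickup and drop through a FlipFlop, tracking IsHeld.
; On destruction it clears the cached player's IsHoldingItem flag.
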(event `/Game/Blueprints/Interfaces/BPI_Interactable.Interact`
  (params (Instigator :type "/Game/Blueprints/Characters/BP_Character_Base Object Reference"))
  (bind _as_bp_player (`self.As BP Player`))
  (bind _asbp_player (cast `/Game/Blueprints/Characters/BP_Player` Instigator))
  (bind _output_get (set `self.As BP Player` _asbp_player))
  (if (`/Game/Blueprints/Characters/BP_Player.HasWrench` _output_get)
    (if (`self.Is Repaired`)
      (`/Engine/EditorBlueprintResources/StandardMacros.FlipFlop`
        (:`A`
          (`/Game/Blueprints/Characters/BP_Player.Pickup box` _as_bp_player)
          (set `self.Is Held` true))
        (:`B`
          (`/Game/Blueprints/Characters/BP_Player.Drop Box` _as_bp_player)
          (set `self.Is Held` false)))
      (else
        (set `self.Is Repaired` true)
        (set `/Game/Blueprints/Characters/BP_Character_Base.Current Row Name` "BoxFixed" _as_bp_player)
        (`/Game/Blueprints/Characters/BP_Character_Base.StartInteraction` _as_bp_player null)
        (`/Game/Blueprints/Characters/BP_Character_Base.ShowDialogueLine` _as_bp_player)))
    (else
      (set `/Game/Blueprints/Characters/BP_Character_Base.Current Row Name` "NoWrench" _as_bp_player)
      (bind _asbp_player_2 (cast `/Game/Blueprints/Characters/BP_Player` (`GameplayStatics.GetPlayerCharacter` 0)))
      (`/Game/Blueprints/Characters/BP_Character_Base.StartInteraction` _asbp_player_2 null)
      (`/Game/Blueprints/Characters/BP_Character_Base.ShowDialogueLine` _asbp_player_2))))

(event `self.ReceiveDestroyed`
  (set `/Game/Blueprints/Characters/BP_Player.IsHoldingItem` false (`self.As BP Player`)))

(fn `ShowNextLine`
  (returns (HasNextLine :type Boolean))
  (return false))

(fn `UserConstructionScript`)