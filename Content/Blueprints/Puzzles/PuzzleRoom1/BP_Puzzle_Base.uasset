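; Base puzzle prop that shows data-table dialogue from the speaker "Popcorn" when the player interacts with it.
; Interact locks player interaction and sends the current DT_Dialogue row to the GameMode's HUD widget, or only plays a sound if no row is set.
; ShowNextLine follows each row's NextRow link and restores the starting row at the chain's end.
; FinishInteraction unlocks the player.
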(event `self.ReceiveBeginPlay`
  ;[1 1 1] This is to cast shadows on the Dialogue Widget
  (`PrimitiveComponent.SetCastShadow` (`self.DialogueIndicator`) false)
  (set `self.Reset Row Name` (`self.Current Row Name`))
  ;[1 1 1] This is to set a reference to Game Instance and Mode for all Props
  (bind _asgi_solar (cast `/Game/Blueprints/GI_Solar` (`GameplayStatics.GetGameInstance`)))
  (set `self.GameInstance` _asgi_solar)
  (bind _asgm_solar (cast `/Game/Blueprints/GM_Solar` (`GameplayStatics.GetGameMode`)))
  (set `self.GameMode` _asgm_solar))

(event `/Game/Blueprints/Interfaces/BPI_Interactable.Interact`
  (params (Instigator :type "/Game/Blueprints/Characters/BP_Character_Base Object Reference"))
  ;[1 1 1] Display Dialogue through Interface
  (if (!= (`self.Current Row Name`) "None")
    (`self.Start Character Interaction` null)
    (`self.StartInteraction` Instigator)
    (`self.ShowDialogueLine`)
    (else
      (`GameplayStatics.PlaySound2D` "/Game/Sounds/S_Ambience_General_Cue.S_Ambience_General_Cue" 1.0 1.0 0.0 null null))))

(event `/Game/Blueprints/Interfaces/BPI_Interactable.FinishInteraction`
  ;[1 1 1] Ends the interaction, the rest is handled on BP Player
  (`self.EndInteraction`))

(fn `EndInteraction`
  (bind _asbp_player (cast `/Game/Blueprints/Characters/BP_Player` (`GameplayStatics.GetPlayerCharacter` 0)))
  (set `/Game/Blueprints/Characters/BP_Character_Base.IsInteractionLocked` false _asbp_player))

(fn `ShowDialogueLine`
  (bind _returnvalue (`|GetDataTableRow` "/Game/DataTables/Dialogue/DT_Dialogue.DT_Dialogue" (`self.Current Row Name`))
    (:`then`
      (bind _asbp_player (cast `/Game/Blueprints/Characters/BP_Player` (`GameplayStatics.GetPlayerCharacter` 0)))
      (bind (_dialoguetext _nextrow) (break `/Game/DataTables/Dialogue/S_DialogueData` _returnvalue))
      (`/Game/UI/Widgets/WBP_HUD.ShowDialogue` (`/Game/Blueprints/GM_Solar.HUDWidget` (`self.GameMode`)) _asbp_player "Popcorn" _dialoguetext)
      (set `self.Next Row` _nextrow)
      (return))))

(fn `ShowNextLine`
  (returns (HasNextLine :type Boolean))
  (if (`KismetStringLibrary.IsEmpty` (`self.Next Row`))
    (set `self.Current Row Name` (`self.Reset Row Name`))
    (else
      (set `self.Current Row Name` (`KismetStringLibrary.Conv_StringToName` (`self.Next Row`)))
      (`self.ShowDialogueLine`)
      (`GameplayStatics.PlaySound2D` "/Engine/VREditor/Sounds/UI/Click_on_Button.Click_on_Button" 1.0 1.0 0.0 null null)))
  (return false))

(fn `Start Character Interaction`
  (params (`Player Character` :type "Actor Object Reference"))
  (bind _asbp_player (cast `/Game/Blueprints/Characters/BP_Player` `Player Character`))
  (`/Game/Blueprints/Characters/BP_Character_Base.StartInteraction` _asbp_player (`self.GetParentActor` _asbp_player)))

(fn `StartInteraction`
  (params (InteractInstigator :type "Actor Object Reference"))
  (bind _asbp_player (cast `/Game/Blueprints/Characters/BP_Player` InteractInstigator))
  (set `/Game/Blueprints/Characters/BP_Character_Base.IsInteractionLocked` true _asbp_player)
  (`GameplayStatics.PlaySound2D` "/Game/Sounds/S_Dialogue_Cue.S_Dialogue_Cue" 0.1 1.0 0.0 null null))

(fn `UserConstructionScript`)