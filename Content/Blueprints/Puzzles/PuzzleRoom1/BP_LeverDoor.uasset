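; Puzzle Room 1 door that opens when six lever flags match a fixed combination of on and off states.
; CheckAnswer tests the flags, then on a match plays a success sound, opens the door and clears the objective text through BP_OBJUpdate.
; A timeline lerps the door's relative Z downward.
; BeginPlay caches a BP_Lever reference, but this graph neither uses it nor sets the flags.
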(event `self.ReceiveBeginPlay`
  (bind _returnvalue (`GameplayStatics.GetActorOfClass` "/Game/Blueprints/Puzzles/PuzzleRoom1/BP_Lever.BP_Lever_C"))
  (set `self.Lever` _returnvalue))

(event `Check Answer`
  (if (and (`self.Lever 1 ON`) (`self.Lever 4 ON`) (`self.Lever 6 ON`) (not (`self.Lever 2 ON`)) (not (`self.Lever 3 ON`)) (not (`self.Lever 5 ON`)))
    (`GameplayStatics.PlaySound2D` "/Game/Sounds/S_CorrectAnswer.S_CorrectAnswer" 1.0 1.0 0.0 null null)
    (`self.Door Open`)
    (bind _returnvalue (`GameplayStatics.GetActorOfClass` "/Game/Blueprints/Objectives/BP_OBJUpdate.BP_OBJUpdate_C"))
    (`/Game/Blueprints/Objectives/BP_OBJUpdate.New Objective` _returnvalue "")))

(event `Door Open`
  (bind (_direction _opening) (`Timeline|Opening`)
    (:`Update`
      (`SceneComponent.K2_SetRelativeLocation` (`self.Door`) (`KismetMathLibrary.MakeVector` 0.0 0.0 (`KismetMathLibrary.Lerp` 265.0 -285.0 _opening)) false false))))

(fn `UserConstructionScript`)