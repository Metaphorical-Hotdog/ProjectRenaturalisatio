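; Interactable lever for Puzzle Room 1, one of six numbered switches that feed the lever door puzzle.
; On BeginPlay it finds the BP_LeverDoor actor; while not Solved, Interact runs the toggle graph matching its LeverNumber.
; Each toggle uses a FlipFlop to set that lever's flag on the door and swap the button's on/off material.
; After each toggle it calls the door's CheckAnswer.
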(event `self.ReceiveBeginPlay`
  (bind _returnvalue (`GameplayStatics.GetActorOfClass` "/Game/Blueprints/Puzzles/PuzzleRoom1/BP_LeverDoor.BP_LeverDoor_C"))
  (set `self.Lever Door Ref` _returnvalue))

(event `/Game/Blueprints/Interfaces/BPI_Interactable.Interact`
  (params (Instigator :type "/Game/Blueprints/Characters/BP_Character_Base Object Reference"))
  (bind _lever_door_ref (`self.Lever Door Ref`))
  (bind _lever_door_ref_2 (`self.Lever Door Ref`))
  (bind _lever_door_ref_3 (`self.Lever Door Ref`))
  (bind _lever_door_ref_4 (`self.Lever Door Ref`))
  (bind _button_lever (`self.Button/Lever`))
  (bind _lever_door_ref_5 (`self.Lever Door Ref`))
  (if (not (`self.Solved`))
    (`|ExecutionSequence`
      (:`then_0`
        (if (== (`self.Lever Number`) 1)
          (`/Engine/EditorBlueprintResources/StandardMacros.FlipFlop`
            (:`A`
              (set `/Game/Blueprints/Puzzles/PuzzleRoom1/BP_LeverDoor.Lever 1 ON` true (`self.Lever Door Ref`))
              (`PrimitiveComponent.SetMaterial` (`self.Button/Lever`) 0 "/Game/Blueprints/Puzzles/PuzzleRoom1/MAT_ButtonON.MAT_ButtonON"))
            (:`B`
              (set `/Game/Blueprints/Puzzles/PuzzleRoom1/BP_LeverDoor.Lever 1 ON` false (`self.Lever Door Ref`))
              (`PrimitiveComponent.SetMaterial` (`self.Button/Lever`) 0 "/Game/Blueprints/Puzzles/PuzzleRoom1/MAT_ButtonOff.MAT_ButtonOff")))
          (`/Game/Blueprints/Puzzles/PuzzleRoom1/BP_LeverDoor.Check Answer` (`self.Lever Door Ref`) :!label _label)))
      (:`then_1`
        (if (== (`self.Lever Number`) 2)
          (`/Engine/EditorBlueprintResources/StandardMacros.FlipFlop`
            (:`A`
              (set `/Game/Blueprints/Puzzles/PuzzleRoom1/BP_LeverDoor.Lever 2 ON` true _lever_door_ref_4)
              (`PrimitiveComponent.SetMaterial` _button_lever 0 "/Game/Blueprints/Puzzles/PuzzleRoom1/MAT_ButtonON.MAT_ButtonON")
              (goto _label))
            (:`B`
              (set `/Game/Blueprints/Puzzles/PuzzleRoom1/BP_LeverDoor.Lever 2 ON` false _lever_door_ref_4)
              (`PrimitiveComponent.SetMaterial` _button_lever 0 "/Game/Blueprints/Puzzles/PuzzleRoom1/MAT_ButtonOff.MAT_ButtonOff")
              (goto _label)))))
      (:`then_2`
        (if (== (`self.Lever Number`) 3)
          (`/Engine/EditorBlueprintResources/StandardMacros.FlipFlop`
            (:`A`
              (set `/Game/Blueprints/Puzzles/PuzzleRoom1/BP_LeverDoor.Lever 3 ON` true _lever_door_ref_5)
              (`PrimitiveComponent.SetMaterial` (`self.Button/Lever`) 0 "/Game/Blueprints/Puzzles/PuzzleRoom1/MAT_ButtonON.MAT_ButtonON")
              (goto _label))
            (:`B`
              (set `/Game/Blueprints/Puzzles/PuzzleRoom1/BP_LeverDoor.Lever 3 ON` false _lever_door_ref_5)
              (`PrimitiveComponent.SetMaterial` (`self.Button/Lever`) 0 "/Game/Blueprints/Puzzles/PuzzleRoom1/MAT_ButtonOff.MAT_ButtonOff")
              (goto _label)))))
      (:`then_3`
        (if (== (`self.Lever Number`) 4)
          (`/Engine/EditorBlueprintResources/StandardMacros.FlipFlop`
            (:`A`
              (set `/Game/Blueprints/Puzzles/PuzzleRoom1/BP_LeverDoor.Lever 4 ON` true _lever_door_ref)
              (`PrimitiveComponent.SetMaterial` (`self.Button/Lever`) 0 "/Game/Blueprints/Puzzles/PuzzleRoom1/MAT_ButtonON.MAT_ButtonON")
              (goto _label))
            (:`B`
              (set `/Game/Blueprints/Puzzles/PuzzleRoom1/BP_LeverDoor.Lever 4 ON` false _lever_door_ref)
              (`PrimitiveComponent.SetMaterial` (`self.Button/Lever`) 0 "/Game/Blueprints/Puzzles/PuzzleRoom1/MAT_ButtonOff.MAT_ButtonOff")
              (goto _label)))))
      (:`then_4`
        (if (== (`self.Lever Number`) 5)
          (`/Engine/EditorBlueprintResources/StandardMacros.FlipFlop`
            (:`A`
              (set `/Game/Blueprints/Puzzles/PuzzleRoom1/BP_LeverDoor.Lever 5 ON` true _lever_door_ref_2)
              (`PrimitiveComponent.SetMaterial` (`self.Button/Lever`) 0 "/Game/Blueprints/Puzzles/PuzzleRoom1/MAT_ButtonON.MAT_ButtonON")
              (goto _label))
            (:`B`
              (set `/Game/Blueprints/Puzzles/PuzzleRoom1/BP_LeverDoor.Lever 5 ON` false _lever_door_ref_2)
              (`PrimitiveComponent.SetMaterial` (`self.Button/Lever`) 0 "/Game/Blueprints/Puzzles/PuzzleRoom1/MAT_ButtonOff.MAT_ButtonOff")
              (goto _label)))))
      (:`then_5`
        (if (== (`self.Lever Number`) 6)
          (`/Engine/EditorBlueprintResources/StandardMacros.FlipFlop`
            (:`A`
              (set `/Game/Blueprints/Puzzles/PuzzleRoom1/BP_LeverDoor.Lever 6 ON` true _lever_door_ref_3)
              (`PrimitiveComponent.SetMaterial` (`self.Button/Lever`) 0 "/Game/Blueprints/Puzzles/PuzzleRoom1/MAT_ButtonON.MAT_ButtonON")
              (goto _label))
            (:`B`
              (set `/Game/Blueprints/Puzzles/PuzzleRoom1/BP_LeverDoor.Lever 6 ON` false _lever_door_ref_3)
              (`PrimitiveComponent.SetMaterial` (`self.Button/Lever`) 0 "/Game/Blueprints/Puzzles/PuzzleRoom1/MAT_ButtonOff.MAT_ButtonOff")
              (goto _label))))))))

(fn `ShowNextLine`
  (returns (HasNextLine :type Boolean))
  (return false))

(fn `UserConstructionScript`)