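; Game mode for Solar that bridges persistent game instance state with the HUD and player.
; On BeginPlay it loads inventory, nature sphere progress and triptych solved flags from GI_Solar, then builds the HUD and has the player check tools and items.
; Small functions write inventory, nature and first-triptych changes back to the game instance.
; Triptych choice events forward to BP_Player.
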(event `self.ReceiveBeginPlay`
  (bind _gameinstance (`self.GameInstance`))
  (bind _asgi_solar (cast `/Game/Blueprints/GI_Solar` (`GameplayStatics.GetGameInstance`)))
  (set `self.GameInstance` _asgi_solar)
  (set `self.Items` (`/Game/Blueprints/GI_Solar.Items` _gameinstance))
  (set `self.NatureSphereMasks` (`/Game/Blueprints/GI_Solar.NatureSphereMasks` _gameinstance))
  (set `self.NatureIndex` (`/Game/Blueprints/GI_Solar.NatureIndex` _gameinstance))
  (`self.UpdateTriptych`)
  (bind _returnvalue (`|CreateWidget` "/Game/UI/Widgets/WBP_HUD.WBP_HUD_C" (`GameplayStatics.GetPlayerController` 0)))
  (bind _output_get (set `self.HUDWidget` _returnvalue))
  (`self.LoadInventory`)
  (`UserWidget.AddToViewport` _output_get 0)
  (set `/Game/UI/Widgets/WBP_SpeechChoice.GameMode` self (`/Game/UI/Widgets/WBP_HUD.WBP_SpeechChoice` (`self.HUDWidget`)))
  (bind _asbp_player (cast `/Game/Blueprints/Characters/BP_Player` (`GameplayStatics.GetPlayerCharacter` 0)))
  (`/Game/Blueprints/Characters/BP_Player.CheckToolsAndItems` _asbp_player (`self.Items`)))

(event `Start Triptych`
  (bind _asbp_player (cast `/Game/Blueprints/Characters/BP_Player` (`GameplayStatics.GetPlayerCharacter` 0)))
  (set `self.Player` _asbp_player))

(event `ChooseFirstTriptych`
  (bind _asbp_player (cast `/Game/Blueprints/Characters/BP_Player` (`GameplayStatics.GetPlayerCharacter` 0)))
  (`/Game/Blueprints/Characters/BP_Player.ChooseFirstTriptych` _asbp_player))

(event `ChooseSecondTriptych`
  (bind _asbp_player (cast `/Game/Blueprints/Characters/BP_Player` (`GameplayStatics.GetPlayerCharacter` 0)))
  (`/Game/Blueprints/Characters/BP_Player.ChooseSecondTriptych` _asbp_player))

(event `ChooseThirdTriptych`
  (bind _asbp_player (cast `/Game/Blueprints/Characters/BP_Player` (`GameplayStatics.GetPlayerCharacter` 0)))
  (`/Game/Blueprints/Characters/BP_Player.ChooseThirdTriptych` _asbp_player))

(fn `IncrementNatureIndex`
  (bind _natureindex (`self.NatureIndex`))
  (`/Engine/EditorBlueprintResources/StandardMacros.IncrementInt` _natureindex
    (:`  `
      (set `/Game/Blueprints/GI_Solar.NatureIndex` _natureindex (`self.GameInstance`)))))

(fn `LoadInventory`
  (`/Game/UI/Widgets/WBP_Inventory.LoadInventory` (`/Game/UI/Widgets/WBP_HUD.WBP_Inventory` (`self.HUDWidget`)) (`self.Items`)))

(fn `SaveFirstTriptych`
  (bind _output_get (set `self.IsFirstTriptychSolved` true))
  (set `/Game/Blueprints/GI_Solar.FirstTriptychSolved` _output_get (`self.GameInstance`)))

(fn `UpdateInventoryData`
  (set `/Game/Blueprints/GI_Solar.Items` (`self.Items`) (`self.GameInstance`)))

(fn `UpdateNatureData`
  (set `/Game/Blueprints/GI_Solar.NatureSphereMasks` (`self.NatureSphereMasks`) (`self.GameInstance`)))

(fn `UpdateTriptych`
  (bind _gameinstance (`self.GameInstance`))
  (set `self.IsFirstTriptychSolved` (`/Game/Blueprints/GI_Solar.FirstTriptychSolved` _gameinstance))
  (set `self.IsSecondTriptychSolved` (`/Game/Blueprints/GI_Solar.SecondTriptychSolved` _gameinstance))
  (set `self.IsThirdTriptychSolved` (`/Game/Blueprints/GI_Solar.ThirdTriptychSolved` _gameinstance)))

(fn `UserConstructionScript`
  (`KismetArrayLibrary.Array_Resize` (`self.Items`) 15))